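; EnemyBase_BP is an enemy base Blueprint that displays the enemy's health on a floating health bar widget.
; Every Tick it casts the Widget component's user widget to FloatingHealthBar_WB and sets the progress bar from GetHealthPercent.
; Logic to rotate the widget toward the player camera is present but unconnected, so it never runs.
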(event `self.ReceiveTick`
  (params (DeltaSeconds :type "Float (single-precision)"))
  ;[1 1 1] EnemyHealthBar update
  (bind _asfloating_health_bar_wb (cast `/Game/UI/HUD/FloatingHealthBar_WB` (`WidgetComponent.GetUserWidgetObject` (`self.Widget`))))
  (`ProgressBar.SetPercent` (`/Game/UI/HUD/FloatingHealthBar_WB.HealthBar` _asfloating_health_bar_wb) (`self.GetHealthPercent`)))

(fn `UserConstructionScript`)