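; Physics-driven torch that can be picked up and dropped, starts lit or unlit, and burns out after being ignited.
; Ignite enables fire particles and looping sound, then starts two timelines driving light intensity and emissive material for flare-up and burn-out.
; Overlapping a TorchStatic_BP spreads flame either way, and a lit torch re-ignites itself, restarting its burn.
; Pickup and drop toggle physics and collision on the mesh.
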(event `self.FireSound.OnAudioFinished`
  (if (`self.IsLit`)
    (`AudioComponent.Play` (`self.FireSound`) 0.0)))

(event `Increase Light`
  ;[1 1 1] LIght Intensity
  (bind (_direction _light_intensity _material_emission) (`Timeline|Change Light` :`NewTime` 0.0 :!via `PlayFromStart`)
    (:`Update`
      (`LightComponent.SetIntensity` (`self.TorchLight`) _light_intensity)
      (bind _returnvalue (`PrimitiveComponent.CreateDynamicMaterialInstance` (`self.TorchMesh`) 2 null))
      (`MaterialInstanceDynamic.SetScalarParameterValue` _returnvalue "Emissive strength" _material_emission))))

(event `FadeOut`
  (bind (_direction _burnoutintensity _burnoutemmision) (`Timeline|BurnOut` :`NewTime` 0.0 :!via `PlayFromStart`)
    (:`Update`
      (`LightComponent.SetIntensity` (`self.TorchLight`) _burnoutintensity)
      (bind _returnvalue (`PrimitiveComponent.CreateDynamicMaterialInstance` (`self.TorchMesh`) 2 null))
      (`MaterialInstanceDynamic.SetScalarParameterValue` _returnvalue "Emissive strength" _burnoutemmision))
    (:`Finished`
      (set `self.IsLit` false)
      (`ActorComponent.Deactivate` (`self.FireParticle`))
      (`PrimitiveComponent.SetMaterial` (`self.TorchMesh`) 2 "/Game/Materials/M_PaintedWood.M_PaintedWood"))))

(event `self.ReceiveBeginPlay`
  ;[1 1 1] Can start in Ignite or extinguish modus
  (`self.Initialize` (`self.TorchMesh`))
  (`PrimitiveComponent.SetSimulatePhysics` (`self.TorchMesh`) true)
  (if (`self.IsLit`)
    (`self.Ignite`)
    (else
      (`self.Extinguish`))))

(event `self.PickUpTorch`
  ;[1 1 1] Pickup/Drop
  (set `self.IsHeld` true)
  (`PrimitiveComponent.SetSimulatePhysics` (`self.TorchMesh`) false)
  (`PrimitiveComponent.SetCollisionEnabled` (`self.TorchMesh`) "NoCollision"))

(event `self.DropTorch`
  ;[1 1 1] Pickup/Drop
  (set `self.IsHeld` false)
  (`PrimitiveComponent.SetCollisionEnabled` (`self.TorchMesh`) "QueryAndPhysics")
  (`PrimitiveComponent.SetSimulatePhysics` (`self.TorchMesh`) true))

(event `self.IgniteOverlap.OnComponentBeginOverlap`
  (params (OverlappedComponent :type "PrimitiveComponent Object Reference") (OtherActor :type "Actor Object Reference") (OtherComp :type "PrimitiveComponent Object Reference") (OtherBodyIndex :type Integer) (bFromSweep :type Boolean) (SweepResult :type "HitResult Structure (by ref)"))
  ;[1 1 1] Ignite/Extinguish on overlap
  (bind _astorch_static_bp (cast `/Game/Blueprint/TorchStatic_BP` OtherActor))
  (if (`self.IsLit`)
    (`/Game/Blueprint/TorchStatic_BP.Ignite` _astorch_static_bp)
    (`self.Ignite`)
    (elif (`TorchStatic.bIsLit` _astorch_static_bp)
      (`self.Ignite`))))

(fn `Extinguish`
  (`ActorComponent.Deactivate` (`self.FireParticle`))
  (set `self.IsLit` false)
  (`PrimitiveComponent.SetMaterial` (`self.TorchMesh`) 2 "/Game/Materials/M_PaintedWood.M_PaintedWood")
  (`LightComponent.SetIntensity` (`self.TorchLight`) 0.0)
  (`AudioComponent.Stop` (`self.FireSound`)))

(fn `Ignite`
  (bind _fireparticle (`self.FireParticle`))
  (`SceneComponent.SetRelativeScale3D` _fireparticle (0.5 0.5 0.5))
  (`ActorComponent.Activate` _fireparticle false)
  (set `self.IsLit` true)
  (`PrimitiveComponent.SetMaterial` (`self.TorchMesh`) 2 "/Game/Materials/Torch_Inst.Torch_Inst")
  (`self.Increase Light`)
  (`AudioComponent.Play` (`self.FireSound`) 0.0)
  (`self.FadeOut`))

(fn `UserConstructionScript`)