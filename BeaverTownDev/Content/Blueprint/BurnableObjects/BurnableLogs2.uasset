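; BurnableLogs2 is a burnable log actor that catches fire from a lit torch, spreads it and burns away.
; Ignite starts particles and sound, activates a child-actor DamageVolume_BP and sets timers that enable spreading, then destroy the actor.
; While spreading, Tick polls the IgniteOverlap volume and ignites unlit BurnableObjects inside.
; Extinguish stops the effects and clears IsLit, leaving timers and damage volume untouched.
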(event `self.ReceiveBeginPlay`
  (bind _asdamage_volume_bp (cast `/Game/Blueprint/DamageVolume_BP` (`ChildActorComponent.ChildActor` (`self.DamageVolume`))))
  (set `self.DamageVolumeRef` _asdamage_volume_bp)
  (`AudioComponent.Stop` (`self.FireSound`)))

(event `self.ReceiveTick`
  (params (DeltaSeconds :type "Float (single-precision)"))
  (if (`self.bCanSpread`)
    (for _array_element (`PrimitiveComponent.GetOverlappingActors` (`self.IgniteOverlap`) null)
      (bind _asburnable_objects (cast `BurnableObjects` _array_element))
      (if (not (`BurnableObjects.bIsLit` _asburnable_objects))
        (`self.IgniteBurnableObjects` _asburnable_objects)))))

(event `self.IgniteOverlap.OnComponentBeginOverlap`
  (params (OverlappedComponent :type "PrimitiveComponent Object Reference") (OtherActor :type "Actor Object Reference") (OtherComp :type "PrimitiveComponent Object Reference") (OtherBodyIndex :type Integer) (bFromSweep :type Boolean) (SweepResult :type "HitResult Structure (by ref)"))
  (bind _astorch_pickup_bp (cast `/Game/Blueprint/TorchPickup_BP` OtherActor))
  (if (`TorchPickup.IsLit` _astorch_pickup_bp)
    (if (not (`self.bIsLit`))
      (`self.Ignite`))))

(event `Set Timers`
  (`KismetSystemLibrary.K2_SetTimerDelegate` (delegate `Spread`) 2.0)
  (`KismetSystemLibrary.K2_SetTimerDelegate` (delegate `Destroy`) 4.0))

(event `Spread`
  (set `self.bCanSpread` true))

(event `Destroy`
  (`self.K2_DestroyActor`))

(event `self.IgniteBurnableObjects`
  (`self.Ignite`))

(fn `Extinguish`
  (`ActorComponent.Deactivate` (`self.FireParticle`))
  (set `self.bIsLit` false)
  (`AudioComponent.Stop` (`self.FireSound`)))

(fn `Ignite`
  (`SceneComponent.SetRelativeScale3D` (`self.FireParticle`) (0.5 0.5 0.5))
  (`ActorComponent.Activate` (`self.FireParticle`) false)
  (set `self.bIsLit` true)
  (`AudioComponent.Play` (`self.FireSound`) 0.0)
  (`self.Set Timers`)
  (`DamageVolume.SetActivate` (`self.DamageVolumeRef`) true))

(fn `UserConstructionScript`)