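; FellableTree_BP is an interactable tree that topples when its TreeOpen dispatcher fires.
; It binds to TreeOpen on BeginPlay, then plays a falling sound while the FallingTree timeline rolls the Tree component, offset by BaseMesh's relative rotation.
; When the timeline finishes, it plays a low-pitched wood-drop sound and destroys TreeHat.
; A separate PlayChopSound event plays the hit sound, using Trunk's relative location as the sound position.
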(event `self.ReceiveBeginPlay`
  (add `self.TreeOpen` (delegate `TreeOpen_Event_0`)))

(event `TreeOpen_Event_0`
  (bind _treehat (`self.TreeHat`))
  (`GameplayStatics.PlaySoundAtLocation` "/Game/Audio/TreeFalling.TreeFalling" (`SceneComponent.K2_GetComponentLocation` (`self.Trunk`)))
  (bind (_direction _treefalling) (`Timeline|FallingTree`)
    (:`Update`
      (`SceneComponent.K2_SetRelativeRotation` (`self.Tree`) (`KismetMathLibrary.ComposeRotators` (`KismetMathLibrary.MakeRotator` _treefalling) (`SceneComponent.RelativeRotation` (`self.BaseMesh`))) false false))
    (:`Finished`
      (`GameplayStatics.PlaySoundAtLocation` "/Game/Audio/DroppingWood.DroppingWood" (`SceneComponent.RelativeLocation` _treehat) (struct) 1000000000.0 0.1 0.1)
      (`ActorComponent.K2_DestroyComponent` _treehat))))

(event `self.PlayChopSound`
  (`GameplayStatics.PlaySoundAtLocation` "/Game/Audio/HitWood.HitWood" (`SceneComponent.RelativeLocation` (`self.Trunk`))))

(fn `UserConstructionScript`)