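; Breakable crate interactable that drops a red, blue or green crystal pickup when broken.
; On BeginPlay it binds to its CrateOpen dispatcher, whose handler checks GetIsBroken and plays either a break or a lighter smash sound.
; When broken, RandomSpawn selects the crystal, which spawns at the mesh's SpawnLocation socket before the crate destroys itself.
; RandomSpawn is only read in this graph, and values outside the three cases leave the crate in place.
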(event `self.ReceiveBeginPlay`
  (add `self.CrateOpen` (delegate `CrateOpen_Event_0`)))

(event `CrateOpen_Event_0`
  (bind _returnvalue (`self.GetIsBroken`))
  (if _returnvalue
    (`GameplayStatics.PlaySoundAtLocation` "/Game/Sounds/66780__kevinkace__crate-break-4.66780__kevinkace__crate-break-4" (`self.K2_GetActorLocation`))
    (if (== (`self.RandomSpawn`) 0)
      (`|SpawnActorFromClass` "/Game/Blueprint/Pickups/PickupCrystalRed.PickupCrystalRed_C" (`KismetMathLibrary.MakeTransform` (`SceneComponent.GetSocketLocation` (`self.Crate`) "SpawnLocation") (`self.K2_GetActorRotation`)) "Undefined" "OverrideRootScale")
      (`self.K2_DestroyActor`)
      (elif (== (`self.RandomSpawn`) 1)
        (`|SpawnActorFromClass` "/Game/Blueprint/Pickups/PickupCrystalBlue.PickupCrystalBlue_C" (`KismetMathLibrary.MakeTransform` (`SceneComponent.GetSocketLocation` (`self.Crate`) "SpawnLocation") (`self.K2_GetActorRotation`)) "Undefined" "OverrideRootScale")
        (`self.K2_DestroyActor`)
        (elif (== (`self.RandomSpawn`) 2)
          (`|SpawnActorFromClass` "/Game/Blueprint/Pickups/PickupCrystalGreen.PickupCrystalGreen_C" (`KismetMathLibrary.MakeTransform` (`SceneComponent.GetSocketLocation` (`self.Crate`) "SpawnLocation") (`self.K2_GetActorRotation`)) "Undefined" "OverrideRootScale")
          (`self.K2_DestroyActor`))))
    (else
      (`GameplayStatics.PlaySoundAtLocation` "/Game/Sounds/31622__srehpog__light-crate-smash1.31622__srehpog__light-crate-smash1" (`self.K2_GetActorLocation`)))))

(fn `UserConstructionScript`)