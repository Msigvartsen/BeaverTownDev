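; Interactable chest that swings its lid open and closed and grants the player the wooden key.
; On BeginPlay it binds handlers to its ChestOpen and ChestClose dispatchers, which play or reverse a timeline.
; The timeline rotates DerivedMesh relative to the base mesh's rotation and triggers a sound from an event track.
; Every timeline update, in either direction, also sets the WoodenKey flag on MainGameInstance.
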(event `self.ReceiveBeginPlay`
  (add `self.ChestOpen` (delegate `ChestOpen_Event_0`))
  (add `self.ChestClose` (delegate `ChestClose_Event_0`)))

(event `ChestOpen_Event_0`
  (bind (_direction _openlock) (`Timeline|Timeline_0` :!label _label)
    (:`Update`
      (`SceneComponent.K2_SetRelativeRotation` (`self.DerivedMesh`) (`KismetMathLibrary.ComposeRotators` (`KismetMathLibrary.MakeRotator` _openlock) (`KismetMathLibrary.MakeRotator` (.roll (`SceneComponent.RelativeRotation` (`self.BaseMesh`))) (.pitch (`SceneComponent.RelativeRotation` (`self.BaseMesh`))) (+ (.yaw (`SceneComponent.RelativeRotation` (`self.BaseMesh`))) -90.0))) false false)
      (bind _asmain_game_instance (cast `MainGameInstance` (`GameplayStatics.GetGameInstance`)))
      (`MainGameInstance.SetWoodenKey` _asmain_game_instance true))
    (:`PlaySound`
      (`GameplayStatics.PlaySoundAtLocation` "/Game/Audio/DoorSound2.DoorSound2" (`self.K2_GetActorLocation`) (struct) 5.0 1.0 1.0))))

(event `ChestClose_Event_0`
  (goto _label :!via `Reverse`))

(fn `UserConstructionScript`)