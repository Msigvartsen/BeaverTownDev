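; BurnableWood is a wooden actor that catches fire from a lit TorchPickup_BP entering its IgniteOverlap, then spreads fire and burns away.
; Ignite starts the fire particle and sound, then sets timers that enable spreading and later destroy the actor.
; While spreading is enabled, Tick ignites any unlit BurnableWood overlapping IgniteOverlap, creating a delayed chain reaction.
; Extinguish stops the effects and clears the lit flag, but leaves spreading and timers untouched.
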(event `self.ReceiveTick`
  (params (DeltaSeconds :type "Float (single-precision)"))
  (if (`self.CanSpread`)
    (for _array_element (`PrimitiveComponent.GetOverlappingActors` (`self.IgniteOverlap`) null)
      (bind _asburnable_wood (cast `/Game/Blueprint/BurnableWood` _array_element))
      (if (not (`/Game/Blueprint/BurnableWood.IsLit` _asburnable_wood))
        (`self.Ignite` _asburnable_wood)))))

(event `self.IgniteOverlap.OnComponentBeginOverlap`
  (params (OverlappedComponent :type "PrimitiveComponent Object Reference") (OtherActor :type "Actor Object Reference") (OtherComp :type "PrimitiveComponent Object Reference") (OtherBodyIndex :type Integer) (bFromSweep :type Boolean) (SweepResult :type "HitResult Structure (by ref)"))
  (bind _astorch_pickup_bp (cast `/Game/Blueprint/TorchPickup_BP` OtherActor))
  (if (`TorchPickup.IsLit` _astorch_pickup_bp)
    (if (not (`self.IsLit`))
      (`self.Ignite`))))

(event `Set Timers`
  (`KismetSystemLibrary.K2_SetTimerDelegate` (delegate `Spread`) 2.0)
  (`KismetSystemLibrary.K2_SetTimerDelegate` (delegate `Destroy`) 3.0))

(event `DestroyTimer`)

(event `Spread`
  (set `self.CanSpread` true))

(event `Destroy`
  (`self.K2_DestroyActor`))

(fn `Extinguish`
  (`ActorComponent.Deactivate` (`self.FireParticle`))
  (set `self.IsLit` false)
  (`AudioComponent.Stop` (`self.FireSound`)))

(fn `Ignite`
  (`SceneComponent.SetRelativeScale3D` (`self.FireParticle`) (0.5 0.5 0.5))
  (`ActorComponent.Activate` (`self.FireParticle`) false)
  (set `self.IsLit` true)
  (`AudioComponent.Play` (`self.FireSound`) 0.0)
  (`self.Set Timers`)
  (`self.DestroyTimer`)
  (`KismetSystemLibrary.PrintString` "TEST"))

(fn `UserConstructionScript`)