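; Trigger volume that shows contextual help text on the HUD when the main character enters its box.
; On overlap, while CanShowText is set, it finds the HelpText_WB widget, enables it and copies its two help strings onto MainCharacter_BP.
; With AddTimer, the text hides after a delay and the trigger stops showing it; otherwise any actor ending overlap hides it, leaving the trigger reusable.
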(event `self.Box.OnComponentBeginOverlap`
  (params (OverlappedComponent :type "PrimitiveComponent Object Reference") (OtherActor :type "Actor Object Reference") (OtherComp :type "PrimitiveComponent Object Reference") (OtherBodyIndex :type Integer) (bFromSweep :type Boolean) (SweepResult :type "HitResult Structure (by ref)"))
  (cast `MainCharacter` OtherActor)
  (if (`self.CanShowText`)
    (bind _foundwidgets (`WidgetBlueprintLibrary.GetAllWidgetsOfClass` "/Game/UI/HUD/HelpTExt_WB.HelpText_WB_C"))
    (bind _ashelp_text_wb (cast `/Game/UI/HUD/HelpTExt_WB` (`KismetArrayLibrary.Array_Get` _foundwidgets)))
    (set `/Game/UI/HUD/HelpTExt_WB.CanShowHUD` true _ashelp_text_wb)
    (bind _asmain_character_bp (cast `/Game/Blueprint/MainCharacter_BP` (`GameplayStatics.GetPlayerCharacter` 0)))
    (set `/Game/Blueprint/MainCharacter_BP.HelpText01` (`self.HelpText01`) _asmain_character_bp)
    (set `/Game/Blueprint/MainCharacter_BP.HelpText02` (`self.HelpText02`) _asmain_character_bp)
    (if (`self.AddTimer`)
      (`KismetSystemLibrary.Delay` (`self.TextDespawnTime`))
      (set `/Game/UI/HUD/HelpTExt_WB.CanShowHUD` false _ashelp_text_wb)
      (set `self.CanShowText` false))))

(event `self.ReceiveActorEndOverlap`
  (params (OtherActor :type "Actor Object Reference"))
  (if (not (`self.AddTimer`))
    (bind _foundwidgets (`WidgetBlueprintLibrary.GetAllWidgetsOfClass` "/Game/UI/HUD/HelpTExt_WB.HelpText_WB_C"))
    (bind _ashelp_text_wb (cast `/Game/UI/HUD/HelpTExt_WB` (`KismetArrayLibrary.Array_Get` _foundwidgets)))
    (set `/Game/UI/HUD/HelpTExt_WB.CanShowHUD` false _ashelp_text_wb)))

(fn `UserConstructionScript`)