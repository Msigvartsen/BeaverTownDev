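; HelpTextInWorld_BP is a world-placed help text popup that appears when the player's MainCharacter walks into its overlap volume.
; On BeginPlay it fills LootTextPopup from HelpTextIn and hides it.
; Each tick it rotates the text's pitch and yaw to face the player camera.
; The overlap reveals the text and sets a four-second lifespan, so the actor destroys itself afterward.
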(event `self.ReceiveTick`
  (params (DeltaSeconds :type "Float (single-precision)"))
  (bind (_returnvalue_roll _returnvalue_pitch _returnvalue_yaw) (`KismetMathLibrary.BreakRotator` (`KismetMathLibrary.FindLookAtRotation` (`SceneComponent.K2_GetComponentLocation` (`self.LootTextPopup`)) (`PlayerCameraManager.GetCameraLocation` (`PlayerController.PlayerCameraManager` (`GameplayStatics.GetPlayerController` 0))))))
  (`SceneComponent.K2_SetWorldRotation` (`self.LootTextPopup`) (`KismetMathLibrary.MakeRotator` 0.0 _returnvalue_pitch _returnvalue_yaw) false false))

(event `self.ReceiveBeginPlay`
  (`TextRenderComponent.K2_SetText` (`self.LootTextPopup`) (`self.HelpTextIn`))
  (`SceneComponent.SetVisibility` (`self.LootTextPopup`) false false))

(event `self.Overlap.OnComponentBeginOverlap`
  (params (OverlappedComponent :type "PrimitiveComponent Object Reference") (OtherActor :type "Actor Object Reference") (OtherComp :type "PrimitiveComponent Object Reference") (OtherBodyIndex :type Integer) (bFromSweep :type Boolean) (SweepResult :type "HitResult Structure (by ref)"))
  (cast `MainCharacter` OtherActor)
  (`SceneComponent.SetVisibility` (`self.LootTextPopup`) true false)
  (`self.SetLifeSpan` 4.0)
  (`KismetSystemLibrary.PrintString` "SET VISIBLE"))

(fn `UserConstructionScript`)