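; Main player character Blueprint that manages the game's HUD, pause and death screens.
; BeginPlay adds the HUD and help text widgets to the viewport.
; The Options input opens the pause menu and pauses the game, guarded by a screen-shown flag.
; Tick polls health percent from MainGameInstance and, at zero or below, shows the restart-level widget and pauses the game.
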(event `self.ReceiveBeginPlay`
  ;[1 1 1] Shows HUD
  (bind _returnvalue (`|CreateWidget` "/Game/UI/HUD/HUD_WB.HUD_WB_C"))
  (`UserWidget.AddToViewport` _returnvalue 0)
  (bind _returnvalue_2 (`|CreateWidget` "/Game/UI/HUD/HelpTExt_WB.HelpText_WB_C"))
  (`UserWidget.AddToViewport` _returnvalue_2 0))

(event `InputAction|Options`
  (params (Key :type "Key Structure" :default "AnyKey"))
  ;[1 1 1] Sets up Pause Menu
  (:`Pressed`
    (if (not (`self.IsScreenShown`))
      (bind _returnvalue (`|CreateWidget` "/Game/UI/GUI/PauseMenu_WB.PauseMenu_WB_C"))
      (`UserWidget.AddToViewport` _returnvalue 0)
      (set `self.IsScreenShown` true)
      (`GameplayStatics.SetGamePaused` true))))

(event `self.ReceiveTick`
  (params (DeltaSeconds :type "Float (single-precision)"))
  ;[1 1 1] Checks if the player is dead. Shows death screen
  (bind _asmain_game_instance (cast `MainGameInstance` (`GameplayStatics.GetGameInstance`)))
  (bind _returnvalue (`MainGameInstance.GetHealthPercent` _asmain_game_instance))
  (if (<= _returnvalue 0.0)
    (bind _returnvalue_2 (`|CreateWidget` "/Game/UI/GUI/RestartLevel.RestartLevel_C"))
    (`UserWidget.AddToViewport` _returnvalue_2 0)
    (`GameplayStatics.SetGamePaused` true)))

(fn `UserConstructionScript`)