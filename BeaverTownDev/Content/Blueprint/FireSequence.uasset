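; FireSequence is a fire actor that lights five small particle effects one after another, then spreads to the next fire in a chain.
; BeginFire starts a chain of timers, one per particle, while a timeline drives the fire light's intensity.
; The last step marks it lit, calls BeginFire on NextFireRef and activates its child damage volume.
; EndFire deactivates the particles and damage volume.
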(event `self.ReceiveBeginPlay`
  (`SceneComponent.SetRelativeScale3D` (`self.FireParticles2`) (0.2 0.2 0.2))
  (`SceneComponent.SetRelativeScale3D` (`self.FireParticles3`) (0.2 0.2 0.2))
  (`SceneComponent.SetRelativeScale3D` (`self.FireParticles4`) (0.2 0.2 0.2))
  (`SceneComponent.SetRelativeScale3D` (`self.FireParticles5`) (0.2 0.2 0.2))
  (`SceneComponent.SetRelativeScale3D` (`self.FireParticles1`) (0.2 0.2 0.2))
  (bind _asdamage_volume_bp (cast `/Game/Blueprint/DamageVolume_BP` (`ChildActorComponent.ChildActor` (`self.DamageVolume`))))
  (set `self.DamageVolumeRef` _asdamage_volume_bp))

(event `Begin Fire`
  (`KismetSystemLibrary.K2_SetTimerDelegate` (delegate `Fire1`) (`self.Time`))
  (bind (_direction _light_intensity) (`Timeline|Timeline_0`)
    (:`Update`
      (`LightComponent.SetIntensity` (`self.FireLight`) _light_intensity))))

(event `End Fire`
  (`ActorComponent.Deactivate` (`self.FireParticles1`))
  (`ActorComponent.Deactivate` (`self.FireParticles2`))
  (`ActorComponent.Deactivate` (`self.FireParticles3`))
  (`ActorComponent.Deactivate` (`self.FireParticles4`))
  (`ActorComponent.Deactivate` (`self.FireParticles5`))
  (`DamageVolume.SetActivate` (`self.DamageVolumeRef`) false))

(event `Fire1`
  (`ActorComponent.Activate` (`self.FireParticles1`) false)
  (`KismetSystemLibrary.K2_SetTimerDelegate` (delegate `Fire2`) (`self.Time`)))

(event `Fire2`
  (`ActorComponent.Activate` (`self.FireParticles2`) false)
  (`KismetSystemLibrary.K2_SetTimerDelegate` (delegate `Fire3`) (`self.Time`)))

(event `Fire3`
  (`ActorComponent.Activate` (`self.FireParticles3`) false)
  (`KismetSystemLibrary.K2_SetTimerDelegate` (delegate `Fire4`) (`self.Time`)))

(event `Fire4`
  (`ActorComponent.Activate` (`self.FireParticles4`) false)
  (`KismetSystemLibrary.K2_SetTimerDelegate` (delegate `Fire5`) (`self.Time`)))

(event `Fire5`
  (`ActorComponent.Activate` (`self.FireParticles5`) false)
  (set `self.IsLit` true)
  (`self.Begin Fire` (`self.NextFireRef`))
  (`DamageVolume.SetActivate` (`self.DamageVolumeRef`) true))

(fn `UserConstructionScript`)