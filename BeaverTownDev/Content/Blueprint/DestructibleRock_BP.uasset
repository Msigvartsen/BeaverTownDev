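; Destructible rock actor that breaks apart into smaller throwable rock pickups when its break event is called.
; A separate event plays a stone hit sound at the mesh location.
; BreakRock plays a break sound, destroys the actor, then spawns a configurable number of ThrowableRock_BP actors at random horizontal offsets slightly above its origin, each set to a shared scale value.
; Hit detection and break conditions are left to external callers.
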(event `self.PlayRockHitSound`
  (`GameplayStatics.PlaySoundAtLocation` "/Game/Audio/StoneHit.StoneHit" (`SceneComponent.K2_GetComponentLocation` (`self.BaseMesh`))))

(event `self.BreakRock`
  (bind (_returnvalue_x _returnvalue_y _returnvalue_z) (`KismetMathLibrary.BreakVector` (`self.K2_GetActorLocation`)))
  (bind _returnvalue (`KismetMathLibrary.RandomFloatInRange` -100.0 100.0))
  (bind _scalevalue (`self.ScaleValue`))
  (`GameplayStatics.PlaySoundAtLocation` "/Game/Audio/StoneBreaks2.StoneBreaks2" (`SceneComponent.K2_GetComponentLocation` (`self.BaseMesh`)))
  (`self.K2_DestroyActor`)
  (for _ (range 1 (+ (`self.RocksToSpawn`) 1))
    (bind _returnvalue_2 (`|SpawnActorFromClass` "/Game/Blueprint/ThrowableRock_BP.ThrowableRock_BP_C" (`KismetMathLibrary.Conv_VectorToTransform` (`KismetMathLibrary.MakeVector` (+ _returnvalue_x _returnvalue) (+ _returnvalue_y _returnvalue) (+ _returnvalue_z 10.0))) "Undefined" "OverrideRootScale"))
    (`self.SetActorScale3D` _returnvalue_2 (`KismetMathLibrary.MakeVector` _scalevalue _scalevalue _scalevalue))))

(fn `UserConstructionScript`)