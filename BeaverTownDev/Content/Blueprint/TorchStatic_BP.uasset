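; TorchStatic_BP is a static torch actor that can be lit or extinguished and starts in either state based on IsLit.
; Ignite and Extinguish toggle the particles and swap a mesh material between torch and painted wood.
; A timeline played forward or in reverse fades the point light intensity and dynamic material emission.
; When TriggerFireSequence is set, igniting also begins a referenced fire sequence and starts fire audio, which replays while lit.
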(event `self.Fire2.OnAudioFinished`
  (if (`self.bIsLit`)
    (`AudioComponent.Play` (`self.Fire2`) 0.0)
    (`KismetSystemLibrary.PrintString` "SOUND LOOPED")))

(event `Increase light`
  ;[1 1 1] LIght Intensity
  (bind (_direction _light_intensity _material_emission) (`Timeline|Change Light` :!label _label)
    (:`Update`
      (`LightComponent.SetIntensity` (`self.PointLight`) _light_intensity)
      (bind _returnvalue (`PrimitiveComponent.CreateDynamicMaterialInstance` (`self.StaticMesh`) 2 null))
      (`MaterialInstanceDynamic.SetScalarParameterValue` _returnvalue "Emissive strength" _material_emission))))

(event `Decrease Light`
  ;[1 1 1] LIght Intensity
  (goto _label :!via `Reverse`))

(event `self.ReceiveBeginPlay`
  ;[1 1 1] Can start in Ignite or extinguish modus
  (if (`self.bIsLit`)
    (`self.Ignite`)
    (else
      (`self.Extinguish`))))

(fn `Extinguish`
  (`ActorComponent.Deactivate` (`self.ParticleSystem`))
  (set `self.bIsLit` false)
  (`PrimitiveComponent.SetMaterial` (`self.StaticMesh`) 2 "/Game/Materials/M_PaintedWood.M_PaintedWood")
  (`self.Decrease Light`)
  (`AudioComponent.Stop` (`self.Fire2`)))

(fn `Ignite`
  (`ActorComponent.Activate` (`self.ParticleSystem`) false)
  (set `self.bIsLit` true)
  (`PrimitiveComponent.SetMaterial` (`self.StaticMesh`) 2 "/Game/Materials/Torch_Inst.Torch_Inst")
  (`self.Increase light`)
  (if (`self.TriggerFireSequence`)
    (if (`self.bIsLit`)
      (`/Game/Blueprint/FireSequence.Begin Fire` (`self.FireSequenceRef`))
      (`GameplayStatics.PlaySoundAtLocation` "/Game/Audio/Fire.Fire" (`SceneComponent.RelativeLocation` (`self.PointLight`)))
      (`AudioComponent.SetSound` (`self.Fire2`) "/Game/Audio/Fire.Fire")
      (`AudioComponent.Play` (`self.Fire2`) 0.0))))

(fn `UserConstructionScript`)