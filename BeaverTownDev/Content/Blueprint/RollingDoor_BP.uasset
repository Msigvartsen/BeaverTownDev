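; A rolling stone door that opens from a linked lever or, when no lever is set, once four torches are lit.
; Tick polls these conditions to play the RollDoor timeline, reversing it while the lever is off; the torch path never reverses.
; The timeline adds pitch to the mesh's starting rotation, drives its Y position, and triggers the stone sound, which stops on finish.
; A fifth torch check and the OPEN function are unused stubs.
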(event `self.ReceiveBeginPlay`
  (set `self.DoorRot` (`SceneComponent.RelativeRotation` (`self.StaticMesh`)))
  (set `self.DoorLoc` (`SceneComponent.RelativeLocation` (`self.StaticMesh`)))
  (`AudioComponent.Stop` (`self.StoneSound`)))

(event `self.ReceiveTick`
  (params (DeltaSeconds :type "Float (single-precision)"))
  (bind (_doorloc_x _doorloc_y _doorloc_z) (`KismetMathLibrary.BreakVector` (`self.DoorLoc`)))
  (if (`KismetSystemLibrary.IsValid` (`self.LeverThatOpensDoor`))
    (if (`Interact.bIsOpenEvent` (`self.LeverThatOpensDoor`))
      (bind (_direction _rotate _translate) (`Timeline|RollDoor` :!label _label)
        (:`Update`
          (`SceneComponent.K2_SetRelativeRotation` (`self.StaticMesh`) (`KismetMathLibrary.ComposeRotators` (`KismetMathLibrary.MakeRotator` 0.0 _rotate) (`self.DoorRot`)) false false)
          (`SceneComponent.K2_SetRelativeLocation` (`self.StaticMesh`) (`KismetMathLibrary.MakeVector` _doorloc_x (- _translate _doorloc_y) _doorloc_z) false false))
        (:`Finished`
          (`AudioComponent.Stop` (`self.StoneSound`)))
        (:`PlaySound`
          (`AudioComponent.Play` (`self.StoneSound`) 0.5)))
      (else
        (goto _label :!via `Reverse`)))
    (elif (and (`KismetSystemLibrary.IsValid` (`self.Torch1`)) (`KismetSystemLibrary.IsValid` (`self.Torch2`)) (`KismetSystemLibrary.IsValid` (`self.Torch3`)) (`KismetSystemLibrary.IsValid` (`self.Torch4`)))
      (if (and (`TorchStatic.bIsLit` (`self.Torch1`)) (`TorchStatic.bIsLit` (`self.Torch2`)) (`TorchStatic.bIsLit` (`self.Torch3`)) (`TorchStatic.bIsLit` (`self.Torch4`)))
        (goto _label)))))

(fn `OPEN`)

(fn `UserConstructionScript`)