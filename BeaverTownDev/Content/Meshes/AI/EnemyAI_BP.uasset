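; Enemy AI Blueprint that drives a floating health bar above the enemy.
; Each Tick it casts the widget component to FloatingHealthBar_WB, sets its percent from GetHealthPercent and rotates the bar's pitch and yaw toward the player camera.
; An unconnected branch would write GetIsAggro to the Blackboard's "IsAggro?" key, delaying the false value by a second, but it never runs.
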(event `self.ReceiveTick`
  (params (DeltaSeconds :type "Float (single-precision)"))
  (bind (_returnvalue_roll _returnvalue_pitch _returnvalue_yaw) (`KismetMathLibrary.BreakRotator` (`KismetMathLibrary.FindLookAtRotation` (`SceneComponent.K2_GetComponentLocation` (`self.HealthBar`)) (`PlayerCameraManager.GetCameraLocation` (`PlayerController.PlayerCameraManager` (`GameplayStatics.GetPlayerController` 0))))))
  ;[1 1 1] EnemyHealthBar update
  (bind _asfloating_health_bar_wb (cast `/Game/UI/HUD/FloatingHealthBar_WB` (`WidgetComponent.GetUserWidgetObject` (`self.HealthBar`))))
  (`ProgressBar.SetPercent` (`/Game/UI/HUD/FloatingHealthBar_WB.HealthBar` _asfloating_health_bar_wb) (`self.GetHealthPercent`))
  ;[1 1 1] Set enemy healthbar to follow player camera
  (`SceneComponent.K2_SetWorldRotation` (`self.HealthBar`) (`KismetMathLibrary.MakeRotator` 0.0 _returnvalue_pitch _returnvalue_yaw) false false))

(fn `UserConstructionScript`)